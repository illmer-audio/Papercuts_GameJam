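; BP_DoorInteractionTrigger is a trigger volume that shows an interaction prompt near a door.
; Player pawn overlap adds the PressE widget and sets PlayerIsNearDoor.
; Any actor's end overlap removes that widget and clears the flag.
; Controller prompt creation and the delayed box relocation for random door spawns are disconnected, leaving BeginPlay empty and only a custom event that removes the controller prompt.
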(event `self.ReceiveBeginPlay`
  ;[1 0.9963 0] Moves The CollisionTrigger to the Teddybear at begin of the level. (Necessary if Door spawns random)
)

(event `self.ReceiveActorEndOverlap`
  (params (OtherActor :type "Actor Object Reference"))
  ;[1 0.9595 0.07245] Delete Press E Widget
  (bind _foundwidgets (`WidgetBlueprintLibrary.GetAllWidgetsOfClass` "/Game/FirstPersonBP/HUD/PressE.PressE_C"))
  (`Widget.RemoveFromParent` _foundwidgets)
  (set `self.PlayerIsNearDoor` false))

(event `self.ReceiveActorBeginOverlap`
  (params (OtherActor :type "Actor Object Reference"))
  (if (not (!= OtherActor (`GameplayStatics.GetPlayerPawn` 0)))
    ;[1 0.8803 0] Press E Widget
    (bind _returnvalue (`|CreateWidget` "/Game/FirstPersonBP/HUD/PressE.PressE_C"))
    (`UserWidget.AddToViewport` _returnvalue 0)
    (set `self.PlayerIsNearDoor` true)))

(event `CustomEvent`
  (params (OtherActor :type "Actor Object Reference"))
  ;[1 0.9595 0.07245] Delete Press E Widget
  (bind _foundwidgets (`WidgetBlueprintLibrary.GetAllWidgetsOfClass` "/Game/FirstPersonBP/HUD/PressXOnController.PressXOnController_C"))
  (`Widget.RemoveFromParent` _foundwidgets)
  (set `self.PlayerIsNearDoor` false))

(fn `UserConstructionScript`)