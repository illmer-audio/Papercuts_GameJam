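; BP_BibEndTrigger is a trigger volume that moves the game on to Kuppel_Scene when the player pawn overlaps it.
; It starts a one-second camera fade to white with audio, holds it, then opens the level after a matching delay.
; It also gathers TeddyChildWithoutPhysics actors without using the result.
; An unconnected "Durch Boden Fallen" (fall through floor) snippet disables player collision and nudges the character downward, but never runs.
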(event `self.ReceiveActorBeginOverlap`
  (params (OtherActor :type "Actor Object Reference"))
  (if (not (!= OtherActor (`GameplayStatics.GetPlayerPawn` 0)))
    (`GameplayStatics.GetAllActorsOfClass` "/Game/TriggerVolumes/TeddyChildWithoutPhysics.TeddyChildWithoutPhysics_C")
    (`PlayerCameraManager.StartCameraFade` (`PlayerController.PlayerCameraManager` (`GameplayStatics.GetPlayerController` 0)) 0.0 1.0 1.0 (struct :`R` 1.0 :`G` 1.0 :`B` 1.0 :`A` 1.0) true true)
    (`KismetSystemLibrary.Delay` 1.0)
    (`GameplayStatics.OpenLevel` "Kuppel_Scene")))

(event `self.ReceiveTick`
  (params (DeltaSeconds :type "Float (single-precision)")))

(fn `UserConstructionScript`)