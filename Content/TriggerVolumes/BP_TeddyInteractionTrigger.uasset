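; Trigger volume that marks when the player is near the TestTeddy actor and shows an interaction prompt.
; On BeginPlay it moves its Box to the first TestTeddy's location, passing that world position as a relative target.
; Any actor overlap adds a PressE widget and sets PlayerIsNearTeddy, without filtering for the player.
; End overlap removes top-level PressE widgets and clears the flag.
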(event `self.ReceiveBeginPlay`
  (bind _outactors (`GameplayStatics.GetAllActorsOfClass` "/Game/TriggerVolumes/TestTeddy.TestTeddy_C"))
  (`KismetSystemLibrary.MoveComponentTo` (`self.Box`) (`self.K2_GetActorLocation` (`|GetArrayItem` _outactors)) (struct) false false 0.2 true))

(event `self.ReceiveActorBeginOverlap`
  (params (OtherActor :type "Actor Object Reference"))
  ;[1 0.8803 0] Press E Widget
  (bind _returnvalue (`|CreateWidget` "/Game/FirstPersonBP/HUD/PressE.PressE_C"))
  (`UserWidget.AddToViewport` _returnvalue 0)
  (set `self.PlayerIsNearTeddy` true))

(event `self.ReceiveActorEndOverlap`
  (params (OtherActor :type "Actor Object Reference"))
  ;[1 0.9595 0.07245] Delete Press E Widget
  (bind _foundwidgets (`WidgetBlueprintLibrary.GetAllWidgetsOfClass` "/Game/FirstPersonBP/HUD/PressE.PressE_C"))
  (`Widget.RemoveFromParent` _foundwidgets)
  (set `self.PlayerIsNearTeddy` false))

(event `self.ReceiveTick`
  (params (DeltaSeconds :type "Float (single-precision)")))

(fn `UserConstructionScript`)