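; BP_Ball_Physical is a ball pit ball that gets a random color and is displaced when the player pawn overlaps it.
; The construction script creates a dynamic material instance on the Sphere and randomizes its "Base Color" parameter per instance.
; On overlap, a swept local offset uses the player's world X and Y plus a small constant as the delta, rather than a direction away from the player.
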(event `self.ReceiveActorBeginOverlap`
  (params (OtherActor :type "Actor Object Reference"))
  (bind (_returnvalue_x _returnvalue_y) (`KismetMathLibrary.BreakVector` (`self.K2_GetActorLocation` (`GameplayStatics.GetPlayerPawn` 0))))
  (if (== OtherActor (`GameplayStatics.GetPlayerPawn` 0))
    (`self.K2_AddActorLocalOffset` (`KismetMathLibrary.MakeVector` (+ _returnvalue_x 5.0) (+ _returnvalue_y 5.0)) true)))

(fn `UserConstructionScript`
  ;[1 0.75 0] Je Instanz
  (bind _returnvalue (`PrimitiveComponent.CreateDynamicMaterialInstance` (`self.Sphere`) 0 null "Base Color"))
  (`MaterialInstanceDynamic.SetVectorParameterValue` _returnvalue "Base Color" (`KismetMathLibrary.MakeColor` (`KismetMathLibrary.RandomFloatInRange` 0.0 1.0) (`KismetMathLibrary.RandomFloatInRange` 0.0 1.0) (`KismetMathLibrary.RandomFloatInRange` 0.0 1.0) (`KismetMathLibrary.RandomFloatInRange` 0.0 1.0))))