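; StuhlBP is a chair actor that plays an FMOD impact sound at the hit location when its mesh collides.
; A Gate opens one second after BeginPlay to ignore early hits, and a DoOnce with a short random reset delay throttles repeats.
; The actor's speed maps inversely to the "Velocity" parameter, which is set before each new play call, so it targets the previously stored event instance.
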(event `self.ReceiveBeginPlay`
  (`KismetSystemLibrary.Delay` 1.0)
  (goto _label :!via `Open`))

(event `self.StaticMeshComponent.OnComponentHit`
  (params (HitComponent :type "PrimitiveComponent Object Reference") (OtherActor :type "Actor Object Reference") (OtherComp :type "PrimitiveComponent Object Reference") (NormalImpulse :type "Vector Structure") (Hit :type "HitResult Structure (by ref)"))
  (`/Engine/EditorBlueprintResources/StandardMacros.Gate` true :!label _label
    (:`Exit`
      (`|ExecutionSequence`
        (:`then_0`
          (`/Engine/EditorBlueprintResources/StandardMacros.DoOnce` false :!label _label_2
            (:`Completed`
              (`FMODBlueprintStatics.EventInstanceSetParameter` (stale _returnvalue) "Velocity" (`KismetMathLibrary.MapRangeClamped` (`KismetMathLibrary.VSize` (`self.GetVelocity`)) 200.0 5.0 0.0 6.0))
              (bind _returnvalue (`FMODBlueprintStatics.PlayEventAtLocation` "/Game/FMOD/Events/Props/Chairs/1.1" (`KismetMathLibrary.Conv_VectorToTransform` (`.Location` (`GameplayStatics.BreakHitResult` Hit))))))))
        (:`then_1`
          (`KismetSystemLibrary.Delay` (`KismetMathLibrary.RandomFloatInRange` 0.1 0.2))
          (goto _label_2 :!via `Reset`))))))

(fn `UserConstructionScript`)